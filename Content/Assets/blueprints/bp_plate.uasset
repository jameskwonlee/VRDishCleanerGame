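; Grabbable plate for a VR game that scores points when washed and then disappears.
; PickUp disables physics and attaches it to the given parent; DropOff restores physics, detaches it and adds a small impulse.
; Overlapping any TriggerBox counts as washing: after a delay it plays a sound, adds Score through myVRGamemode and destroys itself.
; BeginPlay binds to the first BP_StartGameButton's ClearAllPlates dispatcher for end-game cleanup with a sound.
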(event OnComponentBeginOverlap(plate_mesh)
  (params (OverlappedComponent :type Primitive%20Component%20Object%20Reference) (OtherActor :type Actor%20Object%20Reference) (OtherComp :type Primitive%20Component%20Object%20Reference) (OtherBodyIndex :type Integer) (bFromSweep :type Boolean) (SweepResult :type Hit%20Result%20Structure%20%28by%20ref%29))
  ;[1 1 1] Washing Plate
  (Utilities|Casting|CastToTriggerBox OtherActor)
  (Utilities|FlowControl|Delay 2.0)
  (Audio|PlaySoundatLocation "/Game/Assets/audio/SC_collect_item_02_Cue.SC_collect_item_02_Cue" (Transformation|GetWorldLocation (Variables|Default|Getplate_mesh)))
  (bind _asmy_vrgamemode (Utilities|Casting|CastTomyVRGamemode (Game|GetGameMode)))
  (Default|AddPoints _asmy_vrgamemode (Variables|Default|GetScore))
  (Actor|DestroyActor))

(event Custom|Cleaned
  ;[1 1 1] Event Dispatcher Clear All Plates at End Game
  (Audio|PlaySoundatLocation "/Game/Assets/audio/SC_happy_collect_item_07_Cue.SC_happy_collect_item_07_Cue" (Transformation|GetWorldLocation (Variables|Default|Getplate_mesh)) "0, 0, 0" 0.2)
  (Actor|DestroyActor))

(event EventDropOff
  ;[1 1 1] DropOffPlate
  (Physics|SetSimulatePhysics (Variables|Default|Getplate_mesh) true)
  (Transformation|DetachFromActor "KeepRelative" "KeepRelative" "KeepRelative")
  (Physics|AddImpulse (Variables|Default|Getplate_mesh) "0,10.000000,15.000000" "None" false))

(event EventPickUp
  (params (ActorToAttachTo :type Scene%20Component%20Object%20Reference))
  ;[1 1 1] PickUpPlate
  (Physics|SetSimulatePhysics (Variables|Default|Getplate_mesh) false)
  (Transformation|AttachComponentToComponent (VehicleSound|GetRootComponent) ActorToAttachTo "None" "KeepWorld" "KeepWorld" "KeepWorld" true))

(event EventBeginPlay
  ;[1 1 1] Event Dispatcher Clear All Plates at End Game
  (bind _outactors (Actor|GetAllActorsOfClass "/Game/Assets/blueprints/bp_StartGameButton.BP_StartGameButton_C"))
  (bind _output_get (Variables|Default|SetClearPlates (Utilities|Array|Get(acopy) _outactors)))
  (EventDispatchers|BindEventtoClearAllPlates _output_get (delegate Custom|Cleaned)))

(fn ConstructionScript)