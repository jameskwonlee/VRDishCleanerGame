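; Plate portal actor that spawns batches of BP_plate at its PortalBox location in two waves.
; The StartGame and SecondWave events each spawn a random number of plates, with a larger range for the second wave.
; Each event first counts all BP_plate actors in the level and skips its batch at the population cap, which is not rechecked during the loop.
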(event Custom|SecondWave
  ;[1 1 1] Second Wave
  (bind _outactors (Actor|GetAllActorsOfClass "/Game/Assets/blueprints/bp_plate.BP_plate_C"))
  (if (< (Utilities|Array|Length _outactors) 120)
    (for _index (range 0 (Math|Random|RandomIntegerinRange 7 12))
      (Game|SpawnActorfromClass "/Game/Assets/blueprints/bp_plate.BP_plate_C" (Math|Conversions|ToTransform(Vector) (Transformation|GetWorldLocation (Variables|Default|GetPortalBox))) "Undefined" 0 0))))

(event Custom|StartGame
  ;[1 1 1] Plate Spawn Primary Wave
  (bind _outactors (Actor|GetAllActorsOfClass "/Game/Assets/blueprints/bp_plate.BP_plate_C"))
  (if (< (Utilities|Array|Length _outactors) 120)
    (for _index (range 0 (Math|Random|RandomIntegerinRange 5 8))
      (Game|SpawnActorfromClass "/Game/Assets/blueprints/bp_plate.BP_plate_C" (Math|Conversions|ToTransform(Vector) (Transformation|GetWorldLocation (Variables|Default|GetPortalBox))) "Undefined" 0 0))))

(fn ConstructionScript)