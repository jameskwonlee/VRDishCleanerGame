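; VR start button that runs a timed plate-wave round when its mesh is overlapped.
; Any overlap hides the start text, resets time and score, and enables game mode tick.
; A VR pawn overlap also starts StartGame and looping SecondWave timers by name on the first BP_platePortal.
; After 35 seconds, it re-sets SecondWave without a time to stop it, clears plates, restores text and disables tick.
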(event OnComponentBeginOverlap(ButtonMesh)
  (params (OverlappedComponent :type Primitive%20Component%20Object%20Reference) (OtherActor :type Actor%20Object%20Reference) (OtherComp :type Primitive%20Component%20Object%20Reference) (OtherBodyIndex :type Integer) (bFromSweep :type Boolean) (SweepResult :type Hit%20Result%20Structure%20%28by%20ref%29))
  ;[1 1 1] Plate Wave Spawn Start Button
  (Development|SetHiddeninGame (Variables|Default|Gettext_StartGame) true false)
  (bind _asmy_vrgamemode (Utilities|Casting|CastTomyVRGamemode (Game|GetGameMode)))
  (Default|ResetTime _asmy_vrgamemode)
  (Default|ResetScore _asmy_vrgamemode)
  (Actor|Tick|SetActorTickEnabled _asmy_vrgamemode true)
  (Utilities|Casting|CastTomyVRPawn OtherActor)
  (bind _outactors (Actor|GetAllActorsOfClass "/Game/Assets/blueprints/bp_platePortal.BP_platePortal_C"))
  ;;[1 1 1] Wave Spawn Sequence
  (Utilities|Time|SetTimerbyFunctionName (Utilities|Array|Get(acopy) _outactors) "StartGame" 0.1)
  (Utilities|Time|SetTimerbyFunctionName (Utilities|Array|Get(acopy) _outactors) "SecondWave" (Math|Random|RandomFloatinRange 5.0 1e+01) true)
  (Audio|PlaySoundatLocation "/Game/Assets/audio/SC_points_ticker_bonus_score_reward_single_03_Cue.SC_points_ticker_bonus_score_reward_single_03_Cue" (Transformation|GetWorldLocation (Variables|Default|GetButtonMesh)) "0, 0, 0" 0.5)
  (Utilities|FlowControl|Delay 35.0)
  (Utilities|Time|SetTimerbyFunctionName (Utilities|Array|Get(acopy) _outactors) "SecondWave" 0.0)
  ;;[1 1 1] Clear Game Area After Finish
  (Default|CallClearAllPlates)
  (Development|SetHiddeninGame (Variables|Default|Gettext_StartGame) false false)
  (bind _asmy_vrgamemode_2 (Utilities|Casting|CastTomyVRGamemode (Game|GetGameMode)))
  (Actor|Tick|SetActorTickEnabled _asmy_vrgamemode_2))

(fn ConstructionScript)